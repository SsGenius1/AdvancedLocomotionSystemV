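; Render actor that displays an equipped cloth item from the inventory system on a parent mesh.
; On BeginPlay it scans DT_Items for the row matching its ID and caches that row's mesh and equipment info.
; It then assigns static and skeletal meshes, applies the relative transform, attaches at the configured bone and slaves the skeletal mesh via master pose.
; The construction script applies the OwnerNoSee setting to both mesh components.
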(event `self.ReceiveBeginPlay`
  ;[0 0 0] Init Cloth Mesh
  (`self.ReadInfo`)
  (`self.InitRenderMesh`))

(fn `InitRenderMesh`
  (bind _mesh_staticmesh (break `/Game/SimpleInventoryComponent/Blueprints/Structs/Item/S_ItemMesh` (`self.Mesh`)))
  (bind (_mesh_staticmesh_2 _mesh_skeletalmesh) (break `/Game/SimpleInventoryComponent/Blueprints/Structs/Item/S_ItemMesh` (`self.Mesh`)))
  (bind (_info_enable _info_masterposeattachtobone _info_relativetransform) (break `/Game/SimpleInventoryComponent/Blueprints/Structs/Item/S_ItemEquipment` (`self.Info`)))
  (bind (_info_enable_2 _info_masterposeattachtobone_2 _info_relativetransform_2 _info_bonename) (break `/Game/SimpleInventoryComponent/Blueprints/Structs/Item/S_ItemEquipment` (`self.Info`)))
  ;[0 0 0] Inits render mesh basing on Info
  (`SceneComponent.K2_SetRelativeTransform` (`self.StaticMesh`) _info_relativetransform false true)
  (`SceneComponent.K2_SetRelativeTransform` (`self.SkeletalMesh`) _info_relativetransform false true)
  (`SkinnedMeshComponent.SetSkinnedAssetAndUpdate` (`self.SkeletalMesh`) _mesh_skeletalmesh true)
  (`StaticMeshComponent.SetStaticMesh` (`self.StaticMesh`) _mesh_staticmesh)
  (`self.K2_AttachToComponent` (`self.ParentMesh`) _info_bonename "KeepRelative" "KeepRelative" "KeepRelative")
  (`SkinnedMeshComponent.SetLeaderPoseComponent` (`self.SkeletalMesh`) (`self.ParentMesh`) true)
  (return))

(fn `ReadInfo`
  (locals (lData :type "/Game/SimpleInventoryComponent/Blueprints/Structs/Item/S_Item Structure"))
  (bind (_ldata_id _ldata_name _ldata_type _ldata_stacksize _ldata_image _ldata_mesh _ldata_description _ldata_information _ldata_equipment) (break `/Game/SimpleInventoryComponent/Blueprints/Structs/Item/S_Item` (`local.lData`)))
  ;[0 0 0] Reads Cloth Mesh Info from DB using ID
  (bind _outrownames (`DataTableFunctionLibrary.GetDataTableRowNames` "/Game/SimpleInventoryComponent/Blueprints/Datatables/DT_Items.DT_Items"))
  (for _array_element _outrownames
    (bind _returnvalue (`|GetDataTableRow` "/Game/SimpleInventoryComponent/Blueprints/Datatables/DT_Items.DT_Items" _array_element)
      (:`then`
        (set `local.lData` _returnvalue)
        (if (== (`.ID_3_1AD321B841473A657F5765B3C0E5D5CD` (break `/Game/SimpleInventoryComponent/Blueprints/Structs/Item/S_Item` _returnvalue)) (`self.ID`))
          (set `self.Mesh` _ldata_mesh)
          (set `self.Info` _ldata_equipment)
          (return))))))

(fn `UserConstructionScript`
  (`PrimitiveComponent.SetOwnerNoSee` (`self.StaticMesh`) (`self.OwnerNoSee`))
  (`PrimitiveComponent.SetOwnerNoSee` (`self.SkeletalMesh`) (`self.OwnerNoSee`)))