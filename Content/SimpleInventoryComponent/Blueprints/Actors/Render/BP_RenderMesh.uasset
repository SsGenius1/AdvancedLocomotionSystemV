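; Render-to-texture actor for the inventory component that shows a skeletal mesh wearing the player's equipped items.
; ChangeMesh sets the mesh, points the scene capture at a new render target and returns a dynamic material displaying it.
; CalculateClothes syncs with the player pawn's equip slots, spawning BP_RenderCloth actors parented to the mesh for missing equipment and destroying those no longer equipped.
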(fn `CalculateClothes`
  (locals (bFlag :type Boolean) (lCurCloth :type "/Game/SimpleInventoryComponent/Blueprints/Actors/Render/BP_RenderCloth Object Reference"))
  ;[0 0 0] Gets caller cloth items
  (bind _component (message `/Game/SimpleInventoryComponent/Blueprints/Interfaces/BPI_GetInventoryComponent.GetInventoryComponent` (`GameplayStatics.GetPlayerPawn` 0)))
  (for _array_element (`/Game/SimpleInventoryComponent/Blueprints/Component/BPC_SIInventoryComponent.EquipSlots` _component)
    ;[0 0 0] The first loop: create all new cloths which don't exist, but should
    (bind _struct (`/Game/SimpleInventoryComponent/Blueprints/Functions/BFL_GlobalFunctions.ItemIDToStruct` (`.ID_2_9F520D934AF0B452E88AD2ADF6688C05` (break `/Game/SimpleInventoryComponent/Blueprints/Structs/Widget/S_Slot` _array_element))))
    (if (`.Enable_12_2AF9BB174A39E55A8483BEAF7E59942C` (break `/Game/SimpleInventoryComponent/Blueprints/Structs/Item/S_ItemEquipment` (`.Equipment_29_F1E6C36D4F858428A391F9A5CF42D4AA` (break `/Game/SimpleInventoryComponent/Blueprints/Structs/Item/S_Item` _struct))))
      (set `local.bFlag` false)
      (for _array_element_2 (`self.Clothes`)
        (bind _id (break `/Game/SimpleInventoryComponent/Blueprints/Structs/Widget/S_Slot` _array_element))
        (if (== (`/Game/SimpleInventoryComponent/Blueprints/Actors/Render/BP_RenderCloth.ID` _array_element_2) _id)
          (set `local.bFlag` true)
          (break)))
      (if (not (`local.bFlag`))
        (bind _returnvalue (`|SpawnActorFromClass` "/Game/SimpleInventoryComponent/Blueprints/Actors/Render/BP_RenderCloth.BP_RenderCloth_C" (`KismetMathLibrary.MakeTransform` (0.0 0.0 0.0)) "Undefined" "OverrideRootScale" null _id (`self.SkeletalMesh`) null))
        (`KismetArrayLibrary.Array_AddUnique` (`self.Clothes`) _returnvalue))))
  ;[0 0 0] The second loop: remove all old clothes which exist but should not
  (for _array_element_3 (`self.Clothes`)
    (set `local.bFlag` false)
    (for _array_element_4 (`/Game/SimpleInventoryComponent/Blueprints/Component/BPC_SIInventoryComponent.EquipSlots` _component)
      (if (== (`.ID_2_9F520D934AF0B452E88AD2ADF6688C05` (break `/Game/SimpleInventoryComponent/Blueprints/Structs/Widget/S_Slot` _array_element_4)) (`/Game/SimpleInventoryComponent/Blueprints/Actors/Render/BP_RenderCloth.ID` _array_element_3))
        (set `local.bFlag` true)
        (break)))
    (if (not (`local.bFlag`))
      (set `local.lCurCloth` _array_element_3)
      (`KismetArrayLibrary.Array_RemoveItem` (`self.Clothes`) (`local.lCurCloth`))
      (`self.K2_DestroyActor` (`local.lCurCloth`))))
  (return))

(fn `ChangeMesh`
  (params (NewMesh :type "SkeletalMesh Object Reference"))
  (returns (Material :type "MaterialInstanceDynamic Object Reference"))
  (locals (lTexture :type "TextureRenderTarget2D Object Reference") (lMaterial :type "MaterialInstanceDynamic Object Reference"))
  (bind _resolution (`self.Resolution`))
  ;[0 0 0] Set New Skeletal Mesh To Render Mesh
  (`SkinnedMeshComponent.SetSkinnedAssetAndUpdate` (`self.SkeletalMesh`) NewMesh false)
  ;[0 0 0] Create new render Texture
  (bind _returnvalue (`KismetRenderingLibrary.CreateRenderTarget2D` _resolution _resolution))
  (bind _output_get (set `local.lTexture` _returnvalue))
  (set `SceneCaptureComponent2D.TextureTarget` _output_get (`self.SceneCaptureComponent2D`))
  ;[0 0 0] Create Material and return it
  (bind _returnvalue_2 (`KismetMaterialLibrary.CreateDynamicMaterialInstance` "/Game/SimpleInventoryComponent/Assets/Materials/Render/M_RenderTarget.M_RenderTarget"))
  (bind _output_get_2 (set `local.lMaterial` _returnvalue_2))
  (`MaterialInstanceDynamic.SetTextureParameterValue` _output_get_2 "RenderTarget" (`local.lTexture`))
  (return (`local.lMaterial`)))

(fn `UserConstructionScript`)