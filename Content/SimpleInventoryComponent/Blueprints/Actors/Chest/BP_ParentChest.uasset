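; Base chest actor for the inventory system, acting as interactable storage that can also process recipes using fuel, furnace-style.
; On BeginPlay the server builds the slot array with starting items and instantiates recipe and fuel objects from class lists.
; When enabled, a self-rescheduling timer swaps fuel items for their outputs and advances every recipe until fuel checks fail.
; Interacting links the chest to the player's inventory component and toggles a HUD message.
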(event `self.ReceiveBeginPlay`
  ;[0 0 0] Begin Play
  (if (`KismetSystemLibrary.IsServer`)
    (`self.GenerateInventory`)
    (`self.GenerateReciepts`)))

(event `/Game/SimpleInventoryComponent/Blueprints/Interfaces/BPI_SIInteraction.Interact`
  (params (Instigator :type "Actor Object Reference"))
  ;[0 0 0] Interact
  (bind _component (message `/Game/SimpleInventoryComponent/Blueprints/Interfaces/BPI_GetInventoryComponent.GetInventoryComponent` Instigator))
  (set `/Game/SimpleInventoryComponent/Blueprints/Component/BPC_SIInventoryComponent.Chest` self _component)
  (`/Game/SimpleInventoryComponent/Blueprints/Component/BPC_SIInventoryComponent.AddChest ( SERVER )` _component self)
  (message `/Game/SimpleInventoryComponent/Blueprints/Interfaces/BPI_SIHUD.SwapVisibility` (`/Game/SimpleInventoryComponent/Blueprints/Functions/BFL_GlobalFunctions.GetSIHUD`)))

(fn `AddItem`
  (params (Item :type "/Game/SimpleInventoryComponent/Blueprints/Structs/Widget/S_Slot Structure"))
  (locals (lQuantity :type Integer) (lStackSize :type Integer) (lFreeSpace :type Integer :default 0) (lCurIndex :type Integer))
  (bind (_id _quantity) (break `/Game/SimpleInventoryComponent/Blueprints/Structs/Widget/S_Slot` Item))
  (bind _item_id (break `/Game/SimpleInventoryComponent/Blueprints/Structs/Widget/S_Slot` (`local.Item`)))
  (bind _item_id_2 (break `/Game/SimpleInventoryComponent/Blueprints/Structs/Widget/S_Slot` (`local.Item`)))
  (bind _item_id_3 (break `/Game/SimpleInventoryComponent/Blueprints/Structs/Widget/S_Slot` (`local.Item`)))
  (bind _item_id_4 (break `/Game/SimpleInventoryComponent/Blueprints/Structs/Widget/S_Slot` (`local.Item`)))
  (bind (_id_2 _quantity_2) (break `/Game/SimpleInventoryComponent/Blueprints/Structs/Widget/S_Slot` (`|GetArrayItem` (`self.Slots`) (`local.lCurIndex`))))
  ;[0 0 0] Add inputed item to chest with given count
  (set `local.lQuantity` _quantity)
  (bind _struct (`/Game/SimpleInventoryComponent/Blueprints/Functions/BFL_GlobalFunctions.ItemIDToStruct` _id))
  (set `local.lStackSize` (`.StackSize_11_2A50F7B94B8330190B54FD9DEF461723` (break `/Game/SimpleInventoryComponent/Blueprints/Structs/Item/S_Item` _struct)))
  (for (_array_element _array_index) (`self.Slots`)
    (set `local.lCurIndex` _array_index)
    (bind (_id_3 _quantity_3) (break `/Game/SimpleInventoryComponent/Blueprints/Structs/Widget/S_Slot` _array_element))
    (if (== _id_3 _item_id)
      (bind _output_get (set `local.lFreeSpace` (- (`local.lStackSize`) _quantity_3)))
      (if (>= _output_get (`local.lQuantity`))
        (`KismetArrayLibrary.Array_Set` (`self.Slots`) (`local.lCurIndex`) (make `/Game/SimpleInventoryComponent/Blueprints/Structs/Widget/S_Slot` _id_2 (+ _quantity_2 (`local.lQuantity`))))
        (return)
        (else
          (set `local.lQuantity` (- (`local.lQuantity`) (`local.lFreeSpace`)))
          (`KismetArrayLibrary.Array_Set` (`self.Slots`) (`local.lCurIndex`) (make `/Game/SimpleInventoryComponent/Blueprints/Structs/Widget/S_Slot` _item_id_2 (`local.lStackSize`)))))))
  (for (_array_element_2 _array_index_2) (`self.Slots`)
    (set `local.lCurIndex` _array_index_2)
    (if (== (`.ID_2_9F520D934AF0B452E88AD2ADF6688C05` (break `/Game/SimpleInventoryComponent/Blueprints/Structs/Widget/S_Slot` _array_element_2)) -1)
      (if (> (`local.lQuantity`) (`local.lStackSize`))
        (`KismetArrayLibrary.Array_Set` (`self.Slots`) (`local.lCurIndex`) (make `/Game/SimpleInventoryComponent/Blueprints/Structs/Widget/S_Slot` _item_id_3 (`local.lStackSize`)))
        (set `local.lQuantity` (- (`local.lQuantity`) (`local.lStackSize`)))
        (else
          (`KismetArrayLibrary.Array_Set` (`self.Slots`) (`local.lCurIndex`) (make `/Game/SimpleInventoryComponent/Blueprints/Structs/Widget/S_Slot` _item_id_4 (`local.lQuantity`)))
          (return)))))
  (return))

(fn `ContainsFuel`
  (returns (Contain :type Boolean) (FuelIndex :type Integer))
  (locals (lCurIndex :type Integer) (bFlag :type Boolean) (bSuperFlag :type Boolean))
  ;[0 0 0] Returns True if chest contains fuel in invenotry from fuel list
  (for (_array_element _array_index) (`self.OFuels`)
    (set `local.lCurIndex` _array_index)
    (set `local.bSuperFlag` true)
    (for _array_element_2 (`/Game/SimpleInventoryComponent/Blueprints/Objects/O_ParentReciept.Taken` _array_element)
      (set `local.bFlag` false)
      (for _array_element_3 (`self.Slots`)
        (if (== (`.ID_2_9F520D934AF0B452E88AD2ADF6688C05` (break `/Game/SimpleInventoryComponent/Blueprints/Structs/Widget/S_Slot` _array_element_3)) (`.ID_2_9F520D934AF0B452E88AD2ADF6688C05` (break `/Game/SimpleInventoryComponent/Blueprints/Structs/Widget/S_Slot` _array_element_2)))
          (set `local.bFlag` true)
          (break)))
      (if (not (`local.bFlag`))
        (set `local.bSuperFlag` false)
        (break)))
    (if (`local.bSuperFlag`)
      (bind _contains (`self.ContainsPlaceForItems` (`/Game/SimpleInventoryComponent/Blueprints/Objects/O_ParentReciept.Given` (`|GetArrayItem` (`self.OReciepts`) (`local.lCurIndex`)))))
      (if _contains
        (return true (`local.lCurIndex`)))))
  (return false (`local.lCurIndex`)))

(fn `ContainsItems`
  (params (Items :type "Array of /Game/SimpleInventoryComponent/Blueprints/Structs/Widget/S_Slot Structure (by ref)"))
  (returns (Contains :type Boolean))
  ;[0 0 0] Returns True if chest contains all inputed items with given count
  (bind _contains (`/Game/SimpleInventoryComponent/Blueprints/Functions/BFL_GlobalFunctions.ContainsItems` (`self.Slots`) Items))
  (return _contains))

(fn `ContainsPlaceForItems`
  (params (Items :type "Array of /Game/SimpleInventoryComponent/Blueprints/Structs/Widget/S_Slot Structure"))
  (returns (Contains :type Boolean))
  ;[0 0 0] Returns True if chest contains place for all inputed items with given count
  (for _array_element Items
    (bind (_id _quantity) (break `/Game/SimpleInventoryComponent/Blueprints/Structs/Widget/S_Slot` _array_element))
    (bind _contains (`/Game/SimpleInventoryComponent/Blueprints/Functions/BFL_GlobalFunctions.ContainsPlaceForItem` _id _quantity (`self.Slots`)))
    (if (not _contains)
      (return false)))
  (return true))

(fn `GenerateInventory`
  ;[0 0 0] Generates inventory with inputed size
  (for _ (range 1 (+ (* (`self.SizeX`) (`self.SizeY`)) 1))
    (`KismetArrayLibrary.Array_Add` (`self.Slots`) (make `/Game/SimpleInventoryComponent/Blueprints/Structs/Widget/S_Slot` -1)))
  (for _array_element (`self.ToAdd`)
    (`self.AddItem` _array_element))
  (return))

(fn `GenerateReciepts`
  ;[0 0 0] Generates reciepts and fuels for chest
  (for _array_element (`self.Reciepts`)
    (bind _returnvalue (`|GenericCreateObject` _array_element self))
    (`KismetArrayLibrary.Array_AddUnique` (`self.OReciepts`) _returnvalue))
  (for _array_element_2 (`self.Fuels`)
    (bind _returnvalue_2 (`|GenericCreateObject` _array_element_2 self))
    (`KismetArrayLibrary.Array_AddUnique` (`self.OFuels`) _returnvalue_2))
  (return))

(fn `ProcessTick`
  (locals (lTime :type Integer :default 0) (lCurRecieptIcon :type Integer :default 0))
  ;[0 0 0] If enabled, looking for fuel. If chest contains fuels, starts tick with fuel cooldown time, and adds progress for all reciepts
  ;;[0 0 0] Looking for and removing fuel
  (bind (_contain _fuelindex) (`self.ContainsFuel`))
  (if _contain
    (bind _output_get (set `local.lCurRecieptIcon` _fuelindex))
    (bind _output (`|GetArrayItem` (`self.OFuels`) _output_get))
    (for _array_element (`/Game/SimpleInventoryComponent/Blueprints/Objects/O_ParentReciept.Taken` _output)
      (`self.RemoveItem` _array_element))
    (for _array_element_2 (`/Game/SimpleInventoryComponent/Blueprints/Objects/O_ParentReciept.Given` _output)
      (`self.AddItem` _array_element_2))
    ;;[0 0 0] Add Progress to reciepts
    (for _array_element_3 (`self.OReciepts`)
      (`/Game/SimpleInventoryComponent/Blueprints/Objects/O_ParentReciept.Add Progress` _array_element_3 (`/Game/SimpleInventoryComponent/Blueprints/Objects/O_ParentReciept.MaxProgress` (`|GetArrayItem` (`self.OFuels`) (`local.lCurRecieptIcon`)))))
    (bind _contain_2 (`self.ContainsFuel`))
    (if _contain_2
      (`KismetSystemLibrary.K2_SetTimer` null "ProcessTick" (`/Game/SimpleInventoryComponent/Blueprints/Objects/O_ParentReciept.CurProgress` (`|GetArrayItem` (`self.OFuels`) (`local.lCurRecieptIcon`))))
      (return)
      (else
        _)))
  (set `self.bEnabled` false)
  (`KismetSystemLibrary.K2_ClearTimer` null "ProcessTick")
  (return))

(fn `RemoveItem`
  (params (Item :type "/Game/SimpleInventoryComponent/Blueprints/Structs/Widget/S_Slot Structure"))
  (locals (lQuantity :type Integer) (lCurIndex :type Integer))
  (bind _item_id (break `/Game/SimpleInventoryComponent/Blueprints/Structs/Widget/S_Slot` (`local.Item`)))
  ;[0 0 0] Remove inputed item from chest with given count
  (set `local.lQuantity` (`.Quantity_4_6386878E490D41738DE938B5DECE9AA5` (break `/Game/SimpleInventoryComponent/Blueprints/Structs/Widget/S_Slot` Item)))
  (for (_array_element _array_index) (`self.Slots`)
    (set `local.lCurIndex` _array_index)
    (bind (_id _quantity) (break `/Game/SimpleInventoryComponent/Blueprints/Structs/Widget/S_Slot` _array_element))
    (if (== _id _item_id)
      (if (> _quantity (`local.lQuantity`))
        (`KismetArrayLibrary.Array_Set` (`self.Slots`) (`local.lCurIndex`) (make `/Game/SimpleInventoryComponent/Blueprints/Structs/Widget/S_Slot` _id (- _quantity (`local.lQuantity`))))
        (set `local.lQuantity` 0)
        (return)
        (else
          (set `local.lQuantity` (- (`local.lQuantity`) _quantity))
          (`KismetArrayLibrary.Array_Set` (`self.Slots`) (`local.lCurIndex`) (make `/Game/SimpleInventoryComponent/Blueprints/Structs/Widget/S_Slot` -1))))))
  (return))

(fn `SwitchEnable`
  (locals (lFuelIndex :type Integer :default 0))
  ;[0 0 0] Switch chest to enabled/disabled
  (bind (_contain _fuelindex) (`self.ContainsFuel`))
  (if _contain
    (set `local.lFuelIndex` _fuelindex)
    (bind _output_get (set `self.bEnabled` (not (`self.bEnabled`))))
    (if _output_get
      (if (`KismetSystemLibrary.IsServer`)
        (`KismetSystemLibrary.K2_SetTimer` null "ProcessTick" (`/Game/SimpleInventoryComponent/Blueprints/Objects/O_ParentReciept.CurProgress` (`|GetArrayItem` (`self.OFuels`) (`local.lFuelIndex`))))
        (return)
        (else
          _))
      (else
        (`KismetSystemLibrary.K2_ClearTimer` null "ProcessTick")))
    (return)
    (else
      (set `self.bEnabled` false)
      (return))))

(fn `UserConstructionScript`)