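; Base world item actor for the inventory system, a physics-enabled pickup that is added to the interacting actor's inventory.
; On construction and BeginPlay it looks up its DT_Items row by ID index to set static and skeletal meshes and offset.
; Interact passes the item to the instigator's inventory component through a server add call.
; Multicast events replicate physics toggling and destruction, and a quantity update to zero destroys the item.
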(fn `EnablePhysic`
  (params (Enable :type Boolean))
  ;[0 0 0] Enable Item Physic
  (if Enable
    (`PrimitiveComponent.SetSimulatePhysics` (`self.StaticMesh`) true)
    (`PrimitiveComponent.SetSimulatePhysics` (`self.SkeletalMesh`) true)
    (return)
    (else
      (`PrimitiveComponent.SetSimulatePhysics` (`self.StaticMesh`) false)
      (`PrimitiveComponent.SetSimulatePhysics` (`self.SkeletalMesh`) false)
      (return))))

(fn `InitMesh`
  ;[0 0 0] Init mesh from Datatable using item ID
  (bind _outrownames (`DataTableFunctionLibrary.GetDataTableRowNames` "/Game/SimpleInventoryComponent/Blueprints/Datatables/DT_Items.DT_Items"))
  (bind _returnvalue (`|GetDataTableRow` "/Game/SimpleInventoryComponent/Blueprints/Datatables/DT_Items.DT_Items" (`|GetArrayItem` _outrownames (`self.ID`)))
    (:`then`
      (bind (_staticmesh _skeletalmesh _offset) (break `/Game/SimpleInventoryComponent/Blueprints/Structs/Item/S_ItemMesh` (`.Mesh_26_D5DDA4EA4F15CCA87585798B26A63704` (break `/Game/SimpleInventoryComponent/Blueprints/Structs/Item/S_Item` _returnvalue))))
      (`StaticMeshComponent.SetStaticMesh` (`self.StaticMesh`) _staticmesh)
      (`SkinnedMeshComponent.SetSkinnedAssetAndUpdate` (`self.SkeletalMesh`) _skeletalmesh true)
      (`SceneComponent.K2_SetRelativeLocation` (`self.StaticMesh`) _offset false true)
      (`SceneComponent.K2_SetRelativeLocation` (`self.SkeletalMesh`) _offset false true)
      (return))
    (:`RowNotFound`
      (return))))

(fn `UpdateQuantity`
  (params (Quantity :type Integer))
  ;[0 0 0] Updates item quantity and removes item if quantity is 0
  (bind _output_get (set `self.Quantity` Quantity))
  (if (<= _output_get 0)
    (`self.Destroy ( MULTICAST )`)
    (return)
    (else
      (return))))

(fn `UserConstructionScript`
  (`self.InitMesh`))