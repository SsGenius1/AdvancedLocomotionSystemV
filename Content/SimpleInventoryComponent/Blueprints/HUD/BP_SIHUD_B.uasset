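; BP_SIHUD_B is a HUD Blueprint for the Simple Inventory system that creates the W_SIHUD widget on begin play, with inventory and equip slots hidden.
; It forwards update and item-info events to that widget and exposes its canvas and a fixed mode enum.
; Swapping visibility refreshes and toggles the inventory, switching mouse cursor and input mode to match.
; Setting an action or split popup removes the previous one of that kind.
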(event `self.ReceiveBeginPlay`
  (bind _w_inventoryhud (`/Game/SimpleInventoryComponent/Blueprints/HUD/W_SIHUD.W_InventoryHUD` (`self.HUD`)))
  ;[0 0 0] Begin Play
  (bind _returnvalue (`|CreateWidget` "/Game/SimpleInventoryComponent/Blueprints/HUD/W_SIHUD.W_SIHUD_C"))
  (bind _output_get (set `self.HUD` _returnvalue))
  (`UserWidget.AddToViewport` _output_get 0)
  (`/Game/SimpleInventoryComponent/Blueprints/Widgets/HUD/W_InventoryHUD.SetVisibilityExpanded` _w_inventoryhud "Hidden")
  (`Widget.SetVisibility` (`/Game/SimpleInventoryComponent/Blueprints/Widgets/HUD/W_InventoryHUD.W_EquipSlots` _w_inventoryhud) "Hidden"))

(event `/Game/SimpleInventoryComponent/Blueprints/Interfaces/BPI_SIHUD.Update`
  ;[0 0 0] Update
  (`/Game/SimpleInventoryComponent/Blueprints/HUD/W_SIHUD.Update` (`self.HUD`)))

(event `/Game/SimpleInventoryComponent/Blueprints/Interfaces/BPI_SIHUD.SwapVisibility`
  ;[0 0 0] Swap Visibility
  (`/Game/SimpleInventoryComponent/Blueprints/HUD/W_SIHUD.Update` (`self.HUD`))
  (`self.SetHUDVisibility`))

(event `/Game/SimpleInventoryComponent/Blueprints/Interfaces/BPI_SIHUD.SetItemInfo`
  (params (Index :type Integer) (Type :type "/Game/SimpleInventoryComponent/Blueprints/Enums/E_SlotType Enum" :default "NewEnumerator0") (Slot :type "/Game/SimpleInventoryComponent/Blueprints/Widgets/Inventory/W_Slot Object Reference") (bDontShow :type Boolean))
  ;[0 0 0] Set Item Info
  (`/Game/SimpleInventoryComponent/Blueprints/Widgets/HUD/W_InventoryHUD.SetItemInfo` (`/Game/SimpleInventoryComponent/Blueprints/HUD/W_SIHUD.W_InventoryHUD` (`self.HUD`)) Index Type Slot bDontShow))

(event `/Game/SimpleInventoryComponent/Blueprints/Interfaces/BPI_SIHUD.SetLastActionPopup`
  (params (Popup :type "/Game/SimpleInventoryComponent/Blueprints/Widgets/Inventory/Popup/W_ItemActionsPopup Object Reference"))
  ;[0 0 0] Set Popup
  (`/Engine/EditorBlueprintResources/StandardMacros.IsValid` (`self.ActionPopup`)
    (:`Is Valid`
      (`Widget.RemoveFromParent` (`self.ActionPopup`)))
    (:`Is Not Valid`
      _))
  (set `self.ActionPopup` Popup))

(event `/Game/SimpleInventoryComponent/Blueprints/Interfaces/BPI_SIHUD.SetLastSplitPopup`
  (params (Popup :type "/Game/SimpleInventoryComponent/Blueprints/Widgets/Inventory/Popup/W_SplitItem Object Reference"))
  ;[0 0 0] Set Popup
  (`/Engine/EditorBlueprintResources/StandardMacros.IsValid` (`self.SplitPopup`)
    (:`Is Valid`
      (`Widget.RemoveFromParent` (`self.SplitPopup`)))
    (:`Is Not Valid`
      _))
  (set `self.SplitPopup` Popup))

(fn `GetHUDCanvas`
  (returns (Canvas :type "CanvasPanel Object Reference"))
  (return (`/Game/SimpleInventoryComponent/Blueprints/Widgets/HUD/W_InventoryHUD.Canvas` (`/Game/SimpleInventoryComponent/Blueprints/HUD/W_SIHUD.W_InventoryHUD` (`self.HUD`)))))

(fn `GetMode`
  (returns (Mode :type "/Game/SimpleInventoryComponent/Blueprints/Enums/E_HUDMode Enum"))
  (return "NewEnumerator1"))

(fn `SetHUDVisibility`
  (locals (lCurVisibility :type Boolean))
  ;[0 0 0] Switch HUD Visibility
  (set `local.lCurVisibility` (`|EnumEquality` (`Widget.GetVisibility` (`/Game/SimpleInventoryComponent/Blueprints/HUD/W_SIHUD.W_InventoryHUD` (`self.HUD`))) "Visible"))
  (`/Game/SimpleInventoryComponent/Blueprints/Widgets/HUD/W_InventoryHUD.SetVisibilityExpanded` (`/Game/SimpleInventoryComponent/Blueprints/HUD/W_SIHUD.W_InventoryHUD` (`self.HUD`)) (select `bool` (`local.lCurVisibility`) :`false` "Visible" :`true` "Hidden" :!type "ESlateVisibility Enum"))
  (set `PlayerController.bShowMouseCursor` (not (`local.lCurVisibility`)) (`GameplayStatics.GetPlayerController` 0))
  (if (`local.lCurVisibility`)
    (`WidgetBlueprintLibrary.SetInputMode_GameOnly` (`GameplayStatics.GetPlayerController` 0))
    (return)
    (else
      (`WidgetBlueprintLibrary.SetInputMode_GameAndUIEx` (`GameplayStatics.GetPlayerController` 0) (`self.HUD`))
      (return))))

(fn `UserConstructionScript`)