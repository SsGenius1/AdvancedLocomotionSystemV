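; BPC_SIParamComponent is a component in the Simple Inventory system that holds health, hunger and thirst values.
; Add functions cap each value at its maximum and keep hunger and thirst at zero or above, while health has no lower clamp.
; Health at or below zero triggers a one-time demo death event that sets the Dead flag and prints a message.
; Server events forward changes to these functions.
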(fn `AddHealth`
  (params (ToAdd :type "Float (double-precision)"))
  ;[0 0 0] Add Health. If it's <= 0 calls death event
  (bind _output_get (set `self.CurHealth` (`KismetMathLibrary.FMin` (+ ToAdd (`self.CurHealth`)) (`self.MaxHealth`))))
  (if (<= _output_get 0.0)
    (if (not (`self.bDead`))
      (`self.DeathEvent`)
      (return)
      (else
        (return)))
    (else
      (return))))

(fn `AddHungry`
  (params (ToAdd :type "Float (double-precision)"))
  ;[0 0 0] Add Hungry
  (set `self.CurHungry` (`KismetMathLibrary.FMax` (`KismetMathLibrary.FMin` (+ ToAdd (`self.CurHungry`)) (`self.MaxHungry`))))
  (return))

(fn `AddThirsty`
  (params (ToAdd :type "Float (double-precision)"))
  ;[0 0 0] Add Thirsty
  (set `self.CurThirsty` (`KismetMathLibrary.FMax` (`KismetMathLibrary.FMin` (+ ToAdd (`self.CurThirsty`)) (`self.MaxThirsty`))))
  (return))

(fn `DeathEvent`
  ;[0 0 0] Demo Death Event
  (set `self.bDead` true)
  (`KismetSystemLibrary.PrintString` "YOU DIED" true true (struct :`R` 1.0 :`A` 1.0) 9999.0)
  (return))