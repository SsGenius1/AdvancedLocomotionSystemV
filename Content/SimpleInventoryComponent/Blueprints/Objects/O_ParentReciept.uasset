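; O_ParentReciept is a base recipe object for the inventory component, converting Taken items into Given items inside the BP_ParentChest that is its outer object.
; AddProgress accumulates progress while the chest holds the Taken items, resetting it when they are missing, then calls TryToProcess.
; At MaxProgress, TryToProcess resets progress, then swaps the items only if the inputs are present and the outputs fit.
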(fn `Add Progress`
  (params (ToAdd :type "Float (double-precision)"))
  (locals (lChest :type "/Game/SimpleInventoryComponent/Blueprints/Actors/Chest/BP_ParentChest Object Reference"))
  ;[0 0 0] Add Progress If Reciepts can be finished
  (bind _asbp_parent_chest (cast `/Game/SimpleInventoryComponent/Blueprints/Actors/Chest/BP_ParentChest` (`KismetSystemLibrary.GetOuterObject` self))
    (:`then`
      (bind _output_get (set `local.lChest` _asbp_parent_chest))
      (bind _contains (`/Game/SimpleInventoryComponent/Blueprints/Actors/Chest/BP_ParentChest.ContainsItems` _output_get (`self.Taken`)))
      (if _contains
        (set `self.CurProgress` (+ (`self.CurProgress`) (`local.ToAdd`)))
        (`self.TryToProcess`)
        (return)
        (else
          (set `self.CurProgress` 0.0)
          (return))))
    (:`CastFailed`
      (`self.TryToProcess`)
      (return))))

(fn `TryToProcess`
  (locals (lChest :type "/Game/SimpleInventoryComponent/Blueprints/Actors/Chest/BP_ParentChest Object Reference"))
  ;[0 0 0] If Progress ready, removes TAKEN items and adds GIVEN items
  (if (>= (`self.CurProgress`) (`self.MaxProgress`))
    (set `self.CurProgress` 0.0)
    (bind _asbp_parent_chest (cast `/Game/SimpleInventoryComponent/Blueprints/Actors/Chest/BP_ParentChest` (`KismetSystemLibrary.GetOuterObject` self))
      (:`then`
        (bind _output_get (set `local.lChest` _asbp_parent_chest))
        (bind _contains (`/Game/SimpleInventoryComponent/Blueprints/Actors/Chest/BP_ParentChest.ContainsItems` _output_get (`self.Taken`)))
        (if _contains
          (bind _contains_2 (`/Game/SimpleInventoryComponent/Blueprints/Actors/Chest/BP_ParentChest.ContainsPlaceForItems` _output_get (`self.Given`)))
          (if _contains_2
            (for _array_element (`self.Taken`)
              (`/Game/SimpleInventoryComponent/Blueprints/Actors/Chest/BP_ParentChest.RemoveItem` (`local.lChest`) _array_element))
            (for _array_element_2 (`self.Given`)
              (`/Game/SimpleInventoryComponent/Blueprints/Actors/Chest/BP_ParentChest.AddItem` (`local.lChest`) _array_element_2))
            (else
              (return)))
          (else
            (return))))
      (:`CastFailed`
        (return)))
    (else
      (return))))